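; Lightning strike area-of-effect actor that marks a ground spot with a warning decal, then triggers after a delay.
; On BeginPlay it snaps to the first Visibility trace hit below AttackTarget, ignoring the target, and spawns the decal there.
; After DelayBeforeStrike it calls Trigger, which is not defined here, and destroys the decal.
; The trace end multiplies the target's Z by -1000 rather than subtracting an offset.
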(event `self.ReceiveBeginPlay`
  (`parent.ReceiveBeginPlay`)
  (`self.Move to Floor`)
  (bind _returnvalue (`GameplayStatics.SpawnDecalAtLocation` "/Game/TopDown/Decals/Decal_AOE_LightningStrike.Decal_AOE_LightningStrike" (25.0 256.0 256.0) (`self.K2_GetActorLocation`)))
  (`KismetSystemLibrary.Delay` (`self.Delay Before Strike`))
  (`self.Trigger`)
  (`/Engine/EditorBlueprintResources/StandardMacros.IsValid` _returnvalue
    (:`Is Valid`
      (`ActorComponent.K2_DestroyComponent` _returnvalue))))

(event `Move to Floor`
  (bind _attack_target (`self.Attack Target`)
    (:`then`
      (bind _returnvalue (`self.K2_GetActorLocation` _attack_target))
      (bind (_outhit _returnvalue_2) (`KismetSystemLibrary.LineTraceSingle` _returnvalue (* _returnvalue (1.0 1.0 -1000.0)) "TraceTypeQuery1" false (`|MakeArray` _attack_target)))
      (if _returnvalue_2
        (`self.K2_SetActorLocation` (`.Location` (`GameplayStatics.BreakHitResult` _outhit)))))
    (:`else`)))

(fn `UserConstructionScript`
  (`parent.UserConstructionScript`))