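; BP_CharBase is a character base Blueprint whose only implemented logic is applying stat buffs.
; ApplyBuff switches on the requested stat to modify dash cooldown, max dashes, health or max health.
; Dash cooldown and max health scale by Delta, while max dashes (truncated) and health add it.
; A max health buff scales current health by the same factor, and no clamping is applied.
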(fn `ApplyBuff`
  (params (StatToBuff :type "/Game/TopDown/Blueprints/BuffSystem/BuffType Enum" :default "NewEnumerator0") (Delta :type "Float (double-precision)" :default 10.0))
  (switch `/Game/TopDown/Blueprints/BuffSystem/BuffType` StatToBuff
    (:`NewEnumerator0`
      (switch `/Game/TopDown/Blueprints/BuffSystem/Stats` "NewEnumerator0"
        (:`NewEnumerator1`
          (set `self.DashCooldown` (* Delta (`self.DashCooldown`))))
        (:`NewEnumerator3`
          (set `self.MaxDashes` (`KismetMathLibrary.FTrunc` (+ (`self.MaxDashes`) Delta))))
        (:`NewEnumerator4`
          (set `self.CurrentHealth` (+ (`self.CurrentHealth`) Delta)))
        (:`NewEnumerator5`
          (set `self.MaxHealth` (* (`self.MaxHealth`) Delta))
          (set `self.CurrentHealth` (* Delta (`self.CurrentHealth`))))))))

(fn `UserConstructionScript`)