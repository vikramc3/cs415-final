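; Invisible enemy that wanders to random reachable points, pinging a sine tone at random intervals.
; A detection sphere reveals it while BP_TopDownCharacter overlaps and hides it on exit.
; Its box overlap calls TakeDamage on that character.
; AnyDamage lowers clamped health; at zero it adds to the player's Score and the GameInstance's EnemiesDefeated, then destroys its SwordRef and itself.
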(event `self.ReceiveBeginPlay`
  (`|ExecutionSequence`
    (:`then_0`
      (`|AIMoveTo` self (`NavigationSystemV1.K2_GetRandomReachablePointInRadius` (`self.K2_GetActorLocation`) 1000.0 null null) null :!label _label
        (:`OnSuccess`
          (`KismetSystemLibrary.Delay` 2.0)
          (goto _label))))
    (:`then_1`
      (`GameplayStatics.PlaySoundAtLocation` "/Engine/EngineSounds/1kSineTonePing.1kSineTonePing" (`self.K2_GetActorLocation`) (struct) 1.0 1.0 0.0 null null null null :!label _label_2)
      (`KismetSystemLibrary.Delay` (`KismetMathLibrary.RandomFloatInRange` 3.0 8.0))
      (goto _label_2))))

(event `self.SphereCollisionDetection.OnComponentBeginOverlap`
  (params (OverlappedComponent :type "PrimitiveComponent Object Reference") (OtherActor :type "Actor Object Reference") (OtherComp :type "PrimitiveComponent Object Reference") (OtherBodyIndex :type Integer) (bFromSweep :type Boolean) (SweepResult :type "HitResult Structure (by ref)"))
  (cast `/Game/TopDown/Blueprints/BP_TopDownCharacter` OtherActor)
  (`self.SetActorHiddenInGame` false))

(event `self.SphereCollisionDetection.OnComponentEndOverlap`
  (params (OverlappedComponent :type "PrimitiveComponent Object Reference") (OtherActor :type "Actor Object Reference") (OtherComp :type "PrimitiveComponent Object Reference") (OtherBodyIndex :type Integer))
  (cast `/Game/TopDown/Blueprints/BP_TopDownCharacter` OtherActor)
  (`self.SetActorHiddenInGame` true))

(event `self.Box.OnComponentBeginOverlap`
  (params (OverlappedComponent :type "PrimitiveComponent Object Reference") (OtherActor :type "Actor Object Reference") (OtherComp :type "PrimitiveComponent Object Reference") (OtherBodyIndex :type Integer) (bFromSweep :type Boolean) (SweepResult :type "HitResult Structure (by ref)"))
  (bind _asbp_top_down_character (cast `/Game/TopDown/Blueprints/BP_TopDownCharacter` OtherActor))
  (`/Game/TopDown/Blueprints/BP_TopDownCharacter.TakeDamage` _asbp_top_down_character 10.0))

(event `self.ReceiveAnyDamage`
  (params (Damage :type "Float (single-precision)") (DamageType :type "DamageType Object Reference") (InstigatedBy :type "Controller Object Reference") (DamageCauser :type "Actor Object Reference"))
  (bind _curr_health (`self.Curr_Health`))
  (`KismetSystemLibrary.PrintString` (`KismetStringLibrary.Conv_DoubleToString` _curr_health))
  (bind _output_get (set `self.Curr_Health` (* (`KismetMathLibrary.FClamp` (- _curr_health Damage) 0.0 100.0) 1.0)))
  (if (<= _output_get 0.0)
    (bind _asbp_top_down_character (cast `/Game/TopDown/Blueprints/BP_TopDownCharacter` (`GameplayStatics.GetPlayerPawn` 0)))
    (set `/Game/TopDown/Blueprints/BP_TopDownCharacter.Score` (+ (`/Game/TopDown/Blueprints/BP_TopDownCharacter.Score` _asbp_top_down_character) 5) _asbp_top_down_character)
    (set `self.isDead` true)
    (bind _asbp_game_instance (cast `/Game/TopDown/Blueprints/BP_GameInstance` (`GameplayStatics.GetGameInstance`)))
    (set `/Game/TopDown/Blueprints/BP_GameInstance.Enemies_Defeated` (+ (`/Game/TopDown/Blueprints/BP_GameInstance.Enemies_Defeated` _asbp_game_instance) 1) _asbp_game_instance)
    (if (`self.isDead`)
      (`self.K2_DestroyActor` (`self.Sword_Ref`))
      (`self.K2_DestroyActor`))))

(fn `UserConstructionScript`)