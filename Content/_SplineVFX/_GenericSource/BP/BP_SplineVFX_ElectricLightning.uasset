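; BP_SplineVFX_ElectricLightning is a damaging electric lightning VFX actor.
; On BeginPlay a timeline, with play rate set from GrowSpeed in the construction script, drives the Niagara "Progress" float.
; Box overlaps apply Damage to each actor other than BP_TopDownCharacter only once, tracked in a HitActors array.
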(event `self.ReceiveBeginPlay`
  (bind (_direction _newtrack_0) (`Timeline|Timeline`)
    (:`Update`
      (`NiagaraComponent.SetVariableFloat` (`self.Niagara`) "Progress" _newtrack_0))))

(event `self.ReceiveTick`
  (params (DeltaSeconds :type "Float (single-precision)")))

(event `self.Box.OnComponentBeginOverlap`
  (params (OverlappedComponent :type "PrimitiveComponent Object Reference") (OtherActor :type "Actor Object Reference") (OtherComp :type "PrimitiveComponent Object Reference") (OtherBodyIndex :type Integer) (bFromSweep :type Boolean) (SweepResult :type "HitResult Structure (by ref)"))
  (cast `/Game/TopDown/Blueprints/BP_TopDownCharacter` OtherActor
    (:`CastFailed`
      (if (not (`KismetArrayLibrary.Array_Contains` (`self.HitActors`) OtherActor))
        (`KismetArrayLibrary.Array_Add` (`self.HitActors`) OtherActor)
        (`GameplayStatics.ApplyDamage` OtherActor (`self.Damage`) null self)))))

(fn `UserConstructionScript`
  (`TimelineComponent.SetPlayRate` (`self.Timeline`) (`self.GrowSpeed`)))